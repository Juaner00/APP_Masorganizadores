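; Player controller that drives BP_CameraPawn with pan, rotate and zoom input.
; Enhanced Input pan and rotate actions send per-frame mouse deltas, axes swapped, to the pawn, while zoom passes its value through.
; BeginPlay caches the pawn and calls ChangeInput, which adds the camera or element mapping context without removing the other.
; Left mouse or touch release fires the OnRelasease dispatcher.
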(event Input|EnhancedActionEvents|EnhancedInputActionIA_Zoom
  (params (ActionValue :type Float%20%28double-precision%29) (ElapsedSeconds :type Float%20%28double-precision%29) (TriggeredSeconds :type Float%20%28double-precision%29) (InputAction :type Input%20Action%20Object%20Reference :default "/Game/Juaner/InputActions/IA_Zoom.IA_Zoom"))
  (Default|Zoom (Variables|Default|GetCameraPawn) ActionValue))

(event Input|EnhancedActionEvents|EnhancedInputActionIA_Rotate
  (params (ActionValue :type Boolean) (ElapsedSeconds :type Float%20%28double-precision%29) (TriggeredSeconds :type Float%20%28double-precision%29) (InputAction :type Input%20Action%20Object%20Reference :default "/Game/Juaner/InputActions/IA_Rotate.IA_Rotate"))
  (bind (_locationx _locationy) (Game|Player|GetMousePosition))
  (:Triggered
    (Variables|Default|SetLastMousePos (Math|Vector2D|MakeVector2D _locationx _locationy))
    (Default|Rotate (Variables|Default|GetCameraPawn) (Math|Vector2D|MakeVector2D (.y (- (Variables|Default|GetInitialMousePos) (Variables|Default|GetLastMousePos))) (.x (- (Variables|Default|GetInitialMousePos) (Variables|Default|GetLastMousePos)))))
    (Variables|Default|SetInitialMousePos (Variables|Default|GetLastMousePos)))
  (:Started
    (Variables|Default|SetInitialMousePos (Math|Vector2D|MakeVector2D _locationx _locationy))))

(event Input|EnhancedActionEvents|EnhancedInputActionIA_Pan
  (params (ActionValue :type Boolean) (ElapsedSeconds :type Float%20%28double-precision%29) (TriggeredSeconds :type Float%20%28double-precision%29) (InputAction :type Input%20Action%20Object%20Reference :default "/Game/Juaner/InputActions/IA_Pan.IA_Pan"))
  (bind (_locationx _locationy) (Game|Player|GetMousePosition))
  (:Triggered
    (Variables|Default|SetLastMousePos (Math|Vector2D|MakeVector2D _locationx _locationy))
    (Default|Pan (Variables|Default|GetCameraPawn) (Math|Vector2D|MakeVector2D (.y (- (Variables|Default|GetInitialMousePos) (Variables|Default|GetLastMousePos))) (.x (- (Variables|Default|GetInitialMousePos) (Variables|Default|GetLastMousePos)))))
    (Variables|Default|SetInitialMousePos (Variables|Default|GetLastMousePos)))
  (:Started
    (Variables|Default|SetInitialMousePos (Math|Vector2D|MakeVector2D _locationx _locationy))))

(event EventBeginPlay
  (bind _asbp_camera_pawn (Utilities|Casting|CastToBP_CameraPawn (Game|Player|GetPlayerPawn 0)))
  (Variables|Default|SetCameraPawn _asbp_camera_pawn)
  (CallFunction|ChangeInput true))

(event Input|MouseEvents|LeftMouseButton
  (params (Key :type Key%20Structure :default "None"))
  (:Released
    (Default|CallOnRelasease)))

(event Input|TouchEvents|Touch1
  (params (Key :type Key%20Structure :default "None"))
  (:Released
    (Default|CallOnRelasease)))

(fn ConstructionScript)

(fn ChangeInput
  (params (IsCameraInput :type Boolean))
  (Input|AddMappingContext (PlayerController|LocalPlayerSubsystems|GetEnhancedInputLocalPlayerSubsystem) (select IsCameraInput "/Game/Juaner/InputActions/IMC_Camera.IMC_Camera" "/Game/Juaner/InputActions/IMC_Element.IMC_Element") 0 "(bIgnoreAllPressedKeysUntilRelease=True,bForceImmediately=False,bNotifyUserSettings=False)"))