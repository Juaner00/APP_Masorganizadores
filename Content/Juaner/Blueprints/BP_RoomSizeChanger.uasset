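; BP_RoomSizeChanger resizes a box room built from six wall, floor and ceiling actors.
; Initialize stores the six actor references for UpdateSize to use.
; UpdateSize places each face at half the room size from the world origin, rotates it and scales it by size divided by 100.
; Each actor switches briefly to Movable for the teleport and rescale, then returns to Static.
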(fn UpdateSize
  (params (RoomSize :type Vector))
  (bind _returnvalue (/ RoomSize 2))
  (bind _back (Variables|Default|GetBack))
  (bind _left (Variables|Default|GetLeft))
  (bind _right (Variables|Default|GetRight))
  (bind _up (Variables|Default|GetUp))
  (bind _down (Variables|Default|GetDown))
  (bind _front (Variables|Default|GetFront))
  (LocalVariables|SetRoomScale (/ RoomSize 100))
  (LocalVariables|SetHalfSize _returnvalue)
  (LocalVariables|SetInvetedHalfSize (* _returnvalue -1))
  (Utilities|FlowControl|Sequence
    (:then_0
      (Transformation|SetMobility _front "Movable")
      (Transformation|SetActorLocationAndRotation _front (Math|Vector|MakeVector (.x (LocalVariables|GetHalfSize)) 0.0 0.0) "90.000000,0.000000,0.000000" false true)
      (Transformation|SetActorScale3D _front (Math|Vector|MakeVector (.z (LocalVariables|GetRoomScale)) (.y (LocalVariables|GetRoomScale)) 1.0))
      (Transformation|SetMobility _front "Static"))
    (:then_1
      (Transformation|SetMobility _back "Movable")
      (Transformation|SetActorLocationAndRotation _back (Math|Vector|MakeVector (.x (LocalVariables|GetInvetedHalfSize)) 0.0 0.0) "90.000000,180.000000,0.000000" false true)
      (Transformation|SetActorScale3D _back (Math|Vector|MakeVector (.z (LocalVariables|GetRoomScale)) (.y (LocalVariables|GetRoomScale)) 1.0))
      (Transformation|SetMobility _back "Static"))
    (:then_2
      (Transformation|SetMobility _left "Movable")
      (Transformation|SetActorLocationAndRotation _left (Math|Vector|MakeVector 0.0 (.y (LocalVariables|GetInvetedHalfSize)) 0.0) "0.000000,0.000000,90.000000" false true)
      (Transformation|SetActorScale3D _left (Math|Vector|MakeVector (.x (LocalVariables|GetRoomScale)) (.z (LocalVariables|GetRoomScale)) 1.0))
      (Transformation|SetMobility _left "Static"))
    (:then_3
      (Transformation|SetMobility _right "Movable")
      (Transformation|SetActorLocationAndRotation _right (Math|Vector|MakeVector 0.0 (.y (LocalVariables|GetHalfSize)) 0.0) "0.000000,180.000000,90.000000" false true)
      (Transformation|SetActorScale3D _right (Math|Vector|MakeVector (.x (LocalVariables|GetRoomScale)) (.z (LocalVariables|GetRoomScale)) 1.0))
      (Transformation|SetMobility _right "Static"))
    (:then_4
      (Transformation|SetMobility _up "Movable")
      (Transformation|SetActorLocationAndRotation _up (Math|Vector|MakeVector 0.0 0.0 (.z (LocalVariables|GetHalfSize))) "0.000000,180.000000,180.000000" false true)
      (Transformation|SetActorScale3D _up (Math|Vector|MakeVector (.x (LocalVariables|GetRoomScale)) (.y (LocalVariables|GetRoomScale)) 1.0))
      (Transformation|SetMobility _up "Static"))
    (:then_5
      (Transformation|SetMobility _down "Movable")
      (Transformation|SetActorLocationAndRotation _down (Math|Vector|MakeVector 0.0 0.0 (.z (LocalVariables|GetInvetedHalfSize))) "0, 0, 0" false true)
      (Transformation|SetActorScale3D _down (Math|Vector|MakeVector (.x (LocalVariables|GetRoomScale)) (.y (LocalVariables|GetRoomScale)) 1.0))
      (Transformation|SetMobility _down "Static"))))

(fn Initialize
  (params (Front :type Static%20Mesh%20Actor%20Object%20Reference) (Back :type Static%20Mesh%20Actor%20Object%20Reference) (Left :type Static%20Mesh%20Actor%20Object%20Reference) (Right :type Static%20Mesh%20Actor%20Object%20Reference) (Up :type Static%20Mesh%20Actor%20Object%20Reference) (Down :type Static%20Mesh%20Actor%20Object%20Reference))
  (Utilities|FlowControl|Sequence
    (:then_0
      (Variables|Default|SetFront Front))
    (:then_1
      (Variables|Default|SetBack Back))
    (:then_2
      (Variables|Default|SetLeft Left))
    (:then_3
      (Variables|Default|SetRight Right))
    (:then_4
      (Variables|Default|SetUp Up))
    (:then_5
      (Variables|Default|SetDown Down))))