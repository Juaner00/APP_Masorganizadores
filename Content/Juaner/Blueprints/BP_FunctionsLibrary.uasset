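; Blueprint function library of shared shortcuts to the game's core framework objects, plus small UI and size helpers.
; Getters cast to the project's HUD, player controller, game instance, game mode and camera pawn, using player index 0 where a player is needed.
; SetVisible turns booleans into widget visibility, with Collapsed taking priority over Visible or Hidden.
; GetSizeInUnits maps a size option to a fixed number through a Select.
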(fn GetSizeinUnits
  (params (Size :type E_ElementSize%20Enum :default "NewEnumerator0"))
  (return (Utilities|Select :Index Size :NewEnumerator2 0 :NewEnumerator0 50 :NewEnumerator1 75)))

(fn GetHUD
  (bind _asmain_hud (Utilities|Casting|CastToMainHUD (HUD|GetHUD (Game|GetPlayerController 0))))
  (return _asmain_hud))

(fn SetVisible
  (params (Widget :type Widget%20Object%20Reference) (Visible :type Boolean) (Collapsed :type Boolean))
  (Widget|SetVisibility Widget (select Collapsed "Collapsed" (select Visible "Visible" "Hidden"))))

(fn GetMainPlayerController
  (bind _asbp_player_controller (Utilities|Casting|CastToBP_PlayerController (Game|GetPlayerController 0)))
  (return _asbp_player_controller))

(fn GetGameInstance
  (bind _asbp_game_instance (Utilities|Casting|CastToBP_GameInstance (Game|GetGameInstance)))
  (return _asbp_game_instance))

(fn GetMainGameMode
  (bind _asmain_game_mode (Utilities|Casting|CastToMainGameMode (Game|GetGameMode)))
  (return _asmain_game_mode))

(fn GetCameraPawn
  (bind _asbp_camera_pawn (Utilities|Casting|CastToBP_CameraPawn (Game|Player|GetPlayerPawn 0)))
  (return _asbp_camera_pawn))