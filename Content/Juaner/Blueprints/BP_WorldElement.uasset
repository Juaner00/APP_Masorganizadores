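; BP_WorldElement is a clickable world actor whose mesh comes from its ElementInfo data.
; The construction script assigns the mesh and fits a box to its bounds, using a fixed Y extent for one size type.
; Mouse and touch input both fire OnClick, passing itself, and OnRelease dispatchers.
; Helper functions swap the material while recording its type, and toggle custom depth rendering for an outline.
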(event EventActorOnInputTouchBegin
  (params (FingerIndex :type ETouchIndex%20Enum :default "Touch1"))
  (Default|CallOnClick self))

(event EventActorOnInputTouchEnd
  (params (FingerIndex :type ETouchIndex%20Enum :default "Touch1"))
  (Default|CallOnRelease))

(event MouseInput|EventActorOnClicked
  (params (ButtonPressed :type Key%20Structure :default "None"))
  (Default|CallOnClick self))

(event EventActorOnReleased
  (params (ButtonReleased :type Key%20Structure :default "None"))
  (Default|CallOnRelease))

(fn ConstructionScript
  (bind _box (Variables|Default|GetBox))
  (bind _elementinfo (Variables|Default|GetElementInfo))
  (bind _element (Variables|/Game/Juaner/Elements/DA_ElementInfo.DA_ElementInfo_C|GetElement _elementinfo))
  (bind _returnvalue (StaticMesh|GetBounds _element))
  (bind (_origin _boxextent) (Math|BoxSphereBounds|BreakBoxSphereBounds _returnvalue))
  (bind (_x _y _z) (Math|Vector|BreakVector _boxextent))
  (Components|StaticMesh|SetStaticMesh (Variables|Default|GetStaticMesh) _element)
  (Transformation|AddLocalOffset _box _origin false true)
  (Components|Box|SetBoxExtent _box (Math|Vector|MakeVector _x (Math|Float|SelectFloat 12.5 _y (Utilities|Enum|Equal(Enum) (Variables|/Game/Juaner/Elements/DA_ElementInfo.DA_ElementInfo_C|GetSize _elementinfo) "NewEnumerator2")) _z) true))

(fn SetMaterial
  (params (Material :type Material%20Instance%20Object%20Reference) (MaterialType :type E_MaterialType%20Enum :default "NewEnumerator1"))
  (Variables|Default|SetMaterialType MaterialType)
  (Rendering|Material|SetMaterial (Variables|Default|GetStaticMesh) 0 Material))

(fn SetOutline
  (params (Enable :type Boolean))
  (Rendering|SetRenderCustomDepth (Variables|Default|GetStaticMesh) Enable))