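; Room customizer actor that lets the player place, drag, re-material and remove furnishing elements in a resizable room, with save, load and reset.
; Construction scans an asset folder for DA_ElementInfo entries; drag-drop payloads spawn BP_WorldElements that report clicks back for selection.
; Mover, material changer and room size changer components handle grid movement, materials with selection outline, and shell resizing.
; BeginPlay restores the saved room and player; resizing snaps to the grid and updates the HUD.
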(event Custom|CreateElement
  (params (Operation :type Drag%20Drop%20Operation%20Object%20Reference))
  (Utilities|FlowControl|Delay 0.1)
  (Private|CreateElementInternal Operation))

(event Custom|ChangeMaterial
  (params (Material%20Type :type E_MaterialType%20Enum :default "NewEnumerator1"))
  (Default|ChangeMaterial (Variables|Default|GetBP_ElementMaterialChanger) (Variables|Private|GetCurrentElement) Material%20Type))

(event EventBeginPlay
  (bind _hud (CallFunction|GetHUD))
  (bind _bp_elementmover (Variables|Default|GetBP_ElementMover))
  (bind _roomsize (Variables|Default|GetRoomSize))
  (bind _inventory (Variables|/Game/Juaner/Widgets/MainHUD.MainHUD_C|GetInventory _hud))
  (EventDispatchers|BindEventtoOnRelasease (CallFunction|GetMainPlayerController) (EventDispatchers|CreateEvent :!event OnPlayerRelease))
  (Utilities|FlowControl|Delay 0.1)
  (Private|LoadRoom)
  (Default|UpdateSize (Variables|Default|GetBP_RoomSizeChanger) (Variables|Default|GetRoomSize) (Variables|Default|GetPlinthSize))
  (Default|Initialize _bp_elementmover (Variables|Default|GetHorizontalGridSize) (Variables|Default|GetVerticalGridSize))
  (Default|SetRoomSize _bp_elementmover (Variables|Default|GetRoomSize) (Variables|Private|GetInstantiatedElements))
  (Default|SetRoomSizeUI _inventory (.x _roomsize) false)
  (Default|SetRoomSizeUI _inventory (.y _roomsize) true))

(event EventTick
  (params (DeltaSeconds :type Float%20%28single-precision%29))
  (if (Variables|Default|GetIsClicked)
    (Default|MoveElement (Variables|Default|GetBP_ElementMover) (Variables|Private|GetCurrentElement))))

(fn ConstructionScript
  (bind _bp_roomsizechanger (Variables|Default|GetBP_RoomSizeChanger))
  (Utilities|Array|Clear (Variables|Default|GetElements))
  (bind _outassetdata (Class|AssetRegistry|GetAssetsbyPath (Class|AssetRegistryHelpers|GetAssetRegistry) "/Game/Juaner/Elements/Info" false false))
  (Class|AssetRegistryHelpers|SortbyAssetName _outassetdata "Ascending")
  (for _array_element _outassetdata
    (bind _asda_element_info (Utilities|Casting|CastToDA_ElementInfo (Class|AssetRegistryHelpers|GetAsset _array_element)))
    (Utilities|Array|Add (Variables|Default|GetElements) _asda_element_info)
    (Default|Initialize _bp_roomsizechanger (Variables|Room|GetFront) (Variables|Room|GetBack) (Variables|Room|GetLeft) (Variables|Room|GetRight) (Variables|Room|GetUp) (Variables|Room|GetDown) (Variables|Room|GetZocalo1) (Variables|Room|GetZocalo2) (Variables|Room|GetLight))
    (Default|UpdateSize _bp_roomsizechanger (Variables|Default|GetRoomSize) (Variables|Default|GetPlinthSize))))

(fn OnClickedElement
  (params (Element :type BP%20World%20Element%20Object%20Reference))
  (if (!= Element (Variables|Private|GetCurrentElement))
    (Private|SetCurrentElement Element))
  (Variables|Default|SetIsClicked true)
  (Default|CalculateOffset (Variables|Default|GetBP_ElementMover) (Variables|Private|GetCurrentElement)))

(fn OnReleasedElement
  (Variables|Default|SetIsClicked false))

(fn RemoveCurrentElement
  (bind _currentelement (Variables|Private|GetCurrentElement))
  (Utilities|Array|RemoveItem (Variables|Private|GetInstantiatedElements) _currentelement)
  (Actor|DestroyActor _currentelement))

(fn CreateElementInternal
  (params (Operation :type Drag%20Drop%20Operation%20Object%20Reference))
  (bind _asbp_drag_element (Utilities|Casting|CastToBP_DragElement Operation))
  (bind _asda_element_info (Utilities|Casting|CastToDA_ElementInfo (Variables|/Script/UMG.DragDropOperation|GetPayload _asbp_drag_element)))
  (Private|SpawnElement _asda_element_info))

(fn SetCurrentElement
  (params (CurrentElement :type BP%20World%20Element%20Object%20Reference))
  (Utilities|IsValid (Variables|Private|GetCurrentElement)
    (:Is%20Valid
      (Default|ToggleOutline (Variables|Default|GetBP_ElementMaterialChanger) false (Variables|Private|GetCurrentElement)))
    (:Is%20Not%20Valid
      _))
  (bind _output_get (Variables|Private|SetCurrentElement CurrentElement))
  (Utilities|IsValid _output_get
    (:Is%20Valid
      (Default|ToggleOutline (Variables|Default|GetBP_ElementMaterialChanger) true _output_get))
    (:Is%20Not%20Valid
      _))
  (Default|CallOnCurrentElementChanged _output_get)
  (Default|ChangeInput (CallFunction|GetMainPlayerController) (not (Utilities|IsValid (Variables|Private|GetCurrentElement)))))

(fn OnPlayerRelease
  (if (Variables|Default|GetIsClicked)
    (Private|OnReleasedElement)))

(fn ConfirmCurrentElement
  (Private|SetCurrentElement))

(fn SpawnElement
  (params (ElementData :type DA%20Element%20Info%20Object%20Reference))
  (bind _returnvalue (Game|SpawnActorfromClass "/Game/Juaner/Blueprints/BP_WorldElement.BP_WorldElement_C" (Math|Transform|MakeTransform "0, 0, 0" "0, 0, 0" "1.000000,1.000000,1.000000") "Undefined" "MultiplyWithRoot" 0 ElementData 0))
  (Utilities|Array|Add (Variables|Private|GetInstantiatedElements) _returnvalue)
  (EventDispatchers|BindEventtoOnClick _returnvalue (EventDispatchers|CreateEvent :!event OnClickedElement))
  (EventDispatchers|BindEventtoOnRelease _returnvalue (EventDispatchers|CreateEvent :!event OnReleasedElement))
  (Default|SetInitialLocation (Variables|Default|GetBP_ElementMover) _returnvalue)
  (Default|ChangeMaterial (Variables|Default|GetBP_ElementMaterialChanger) _returnvalue (Variables|/Game/Juaner/Elements/DA_ElementInfo.DA_ElementInfo_C|GetMaterial ElementData))
  (Private|SetCurrentElement _returnvalue))

(fn SetInitialState
  (params (Elements :type Array%20of%20S%20Save%20Element%20Data%20Structures))
  (for _array_element Elements
    (Private|SpawnInitialElement (.Element (Utilities|Struct|BreakS_SaveElementData _array_element)) (.MaterialType (Utilities|Struct|BreakS_SaveElementData _array_element)) (.Location (Utilities|Struct|BreakS_SaveElementData _array_element)) (.Rotation (Utilities|Struct|BreakS_SaveElementData _array_element)))))

(fn SpawnInitialElement
  (params (Element :type DA%20Element%20Info%20Object%20Reference) (MaterialType :type E_MaterialType%20Enum :default "NewEnumerator5") (Location :type Vector) (Rotation :type Rotator))
  (bind _returnvalue (Game|SpawnActorfromClass "/Game/Juaner/Blueprints/BP_WorldElement.BP_WorldElement_C" (Math|Transform|MakeTransform Location Rotation "1.000000,1.000000,1.000000") "Undefined" "MultiplyWithRoot" 0 Element 0))
  (Utilities|Array|Add (Variables|Private|GetInstantiatedElements) _returnvalue)
  (Default|ChangeMaterial (Variables|Default|GetBP_ElementMaterialChanger) _returnvalue MaterialType)
  (EventDispatchers|BindEventtoOnClick _returnvalue (EventDispatchers|CreateEvent :!event OnClickedElement))
  (EventDispatchers|BindEventtoOnRelease _returnvalue (EventDispatchers|CreateEvent :!event OnReleasedElement)))

(fn SaveRoom
  (Default|SaveGame (CallFunction|GetGameInstance) (Variables|Private|GetInstantiatedElements) (Variables|Default|GetRoomSize)))

(fn LoadRoom
  (bind (_elements _roomsize _playerlocation _playerlook) (Default|LoadGame (CallFunction|GetGameInstance)))
  (Variables|Default|SetRoomSize (Math|Vector|SelectVector "400.000000,400.000000,240.000000" _roomsize (Math|Vector|VectorIsZero _roomsize)))
  (Private|SetInitialState _elements)
  (Default|LoadPlayer (CallFunction|GetMainPlayerController) _playerlocation _playerlook))

(fn ResetRoom
  (bind _arrayelement (Utilities|Array|ReverseforEachLoop (Variables|Private|GetInstantiatedElements))
    (:LoopBody
      (Actor|DestroyActor _arrayelement))
    (:Completed
      (Utilities|Array|Clear (Variables|Private|GetInstantiatedElements))
      (Private|SetCurrentElement))))

(fn SetRoomSize
  (params (Size :type Float%20%28double-precision%29) (Width :type Boolean))
  (bind _horizontalgridsize (Variables|Default|GetHorizontalGridSize))
  (bind _horizontalgridsize_2 (Variables|Default|GetHorizontalGridSize))
  (bind _returnvalue (/ Size _horizontalgridsize))
  (bind _returnvalue_2 (Math|Float|Round _returnvalue))
  (bind _returnvalue_3 (* _returnvalue_2 _horizontalgridsize_2))
  (bind _output_get (Variables|Default|SetRoomSize (Math|Vector|MakeVector (Math|Float|SelectFloat (.x (Variables|Default|GetRoomSize)) _returnvalue_3 Width) (Math|Float|SelectFloat _returnvalue_3 (.y (Variables|Default|GetRoomSize)) Width) (.z (Variables|Default|GetRoomSize)))))
  (Default|SetRoomSize (Variables|Default|GetBP_ElementMover) _output_get (Variables|Private|GetInstantiatedElements))
  (Default|UpdateSize (Variables|Default|GetBP_RoomSizeChanger) _output_get 0.0)
  (Default|SetRoomSizeUI (Variables|/Game/Juaner/Widgets/MainHUD.MainHUD_C|GetInventory (CallFunction|GetHUD)) _returnvalue_3 Width))

(fn ModifyRoomSize
  (params (Width :type Boolean) (Add :type Boolean))
  (bind _horizontalgridsize (Variables|Default|GetHorizontalGridSize))
  (bind _roomsize (Variables|Default|GetRoomSize))
  (bind _returnvalue (Math|Float|SelectFloat (.y _roomsize) (.x _roomsize) Width))
  (bind _returnvalue_2 (* _horizontalgridsize 2))
  (CallFunction|SetRoomSize (Math|Float|SelectFloat (+ _returnvalue _returnvalue_2) (- _returnvalue _returnvalue_2) Add) Width))