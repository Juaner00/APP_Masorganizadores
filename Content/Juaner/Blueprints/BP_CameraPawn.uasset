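; BP_CameraPawn is a free-moving camera pawn exposing Pan, Rotate and Zoom functions, with no event or input logic of its own.
; Pan offsets the pawn along its local Y/Z plane and Zoom along its local forward axis, each scaled by a multiplier.
; Rotate applies yaw in world space and pitch in local space, then clamps pitch within symmetric limits and zeroes roll.
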(event EventBeginPlay)

(event Collision|EventActorBeginOverlap
  (params (OtherActor :type Actor%20Object%20Reference)))

(event EventTick
  (params (DeltaSeconds :type Float%20%28single-precision%29)))

(fn ConstructionScript)

(fn Pan
  (params (Offset :type Vector%202D%20Structure))
  (bind _panmultiplier (Variables|Default|GetPanMultiplier))
  (bind _returnvalue (* Offset _panmultiplier))
  (Transformation|AddActorLocalOffset (Math|Vector|MakeVector 0.0 (.y _returnvalue) (* (.x _returnvalue) -1)) false false))

(fn Rotate
  (params (Offset :type Vector%202D%20Structure))
  (bind _returnvalue (Transformation|GetActorRotation))
  (bind _rotationmultiplayer (Variables|Default|GetRotationMultiplayer))
  (bind _returnvalue_2 (* Offset _rotationmultiplayer))
  (Class|Actor|AddActorWorldRotation (Math|Rotator|MakeRotator 0.0 0.0 (* (.y _returnvalue_2) -1)))
  (Transformation|AddActorLocalRotation (Math|Rotator|MakeRotator 0.0 (.x _returnvalue_2) 0.0) false false)
  (Transformation|SetActorRelativeRotation (Math|Rotator|MakeRotator 0.0 (Math|Float|ClampAngle (.pitch _returnvalue) -7e+01 7e+01) (.yaw _returnvalue))))

(fn Zoom
  (params (Amount :type Float%20%28double-precision%29))
  (Transformation|AddActorLocalOffset (Math|Vector|MakeVector (* Amount (Variables|Default|GetZoomMultiplier)) 0.0 0.0) false false))