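; BP_ElementMover places and drags elements along the four walls of a rectangular room.
; It intersects a touch or mouse ray with the wall planes to get a position and inward normal.
; CalculateOffset stores the grab offset and wall normal; MoveElement rotates that offset when the wall changes.
; Positions are clamped by room and element bounds, snapped to a size-aware grid, and elements face along the wall normal.
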(event EventBeginPlay)

(fn GetValidRoomPosition
  (params (Element :type BP%20World%20Element%20Object%20Reference) (Initial :type Vector) (NewNormal :type Vector))
  (bind _returnvalue (Class|KismetMathLibrary|VectorRight))
  (bind (_x _y _z) (Math|Vector|BreakVector Initial))
  (bind _roomsize (Variables|Private|GetRoomSize))
  (bind _returnvalue_2 (Math|Vector|VectorGetAbs NewNormal))
  (bind _returnvalue_3 (/ _roomsize 2))
  (bind _elementinfo (Variables|/Game/Juaner/Blueprints/BP_WorldElement.BP_WorldElement_C|GetElementInfo Element))
  (bind (_x_2 _y_2 _z_2) (Math|Vector|BreakVector _returnvalue_3))
  (bind _returnvalue_4 (* _returnvalue_3 -1))
  (bind _returnvalue_5 (Utilities|Operators|EqualEqual _returnvalue_2 _returnvalue 0.0))
  (bind _size (Variables|/Game/Juaner/Elements/DA_ElementInfo.DA_ElementInfo_C|GetSize _elementinfo))
  (bind _returnvalue_6 (StaticMesh|GetBounds (Variables|/Game/Juaner/Elements/DA_ElementInfo.DA_ElementInfo_C|GetElement _elementinfo)))
  (bind (_x_3 _y_3 _z_3) (Math|Vector|BreakVector _returnvalue_4))
  (bind _returnvalue_7 (Utilities|Enum|Equal(Enum) _size "NewEnumerator2"))
  (bind (_origin _boxextent) (Math|BoxSphereBounds|BreakBoxSphereBounds _returnvalue_6))
  (bind (_x_4 _y_4 _z_4) (Math|Vector|BreakVector _boxextent))
  (bind _returnvalue_8 (Math|Float|SelectFloat 0.0 _y_4 _returnvalue_7))
  (bind _returnvalue_9 (Math|Vector|MakeVector _x_4 _returnvalue_8 _z_4))
  (bind _returnvalue_10 (+ _origin _returnvalue_9))
  (bind (_x_5 _y_5 _z_5) (Math|Vector|BreakVector _returnvalue_10))
  (bind _returnvalue_11 (Math|Float|SelectFloat _y_5 0.0 _returnvalue_5))
  (bind _returnvalue_12 (Math|Float|SelectFloat 0.0 _y_5 _returnvalue_5))
  (return (Math|Vector|MakeVector (Math|Float|Clamp(Float) _x (+ _x_3 _returnvalue_11) (- _x_2 _returnvalue_11)) (Math|Float|Clamp(Float) _y (+ _y_3 _returnvalue_12) (- _y_2 _returnvalue_12)) (Math|Float|Clamp(Float) _z _z_3 (- _z_2 _z_5)))))

(fn GetMouseLocation
  (bind _returnvalue (Math|Vector|MakeVector 0.0 -1.0 0.0))
  (bind _returnvalue_2 (Math|Vector|MakeVector 0.0 1.0 0.0))
  (bind _returnvalue_3 (Math|Vector|MakeVector 1.0 0.0 0.0))
  (bind _returnvalue_4 (Math|Vector|MakeVector -1.0 0.0 0.0))
  (bind _playercontroller (CallFunction|GetMainPlayerController))
  (bind _roomsize (Variables|Private|GetRoomSize))
  (bind (_locationx _locationy _biscurrentlypressed) (Class|PlayerController|GetInputTouchState _playercontroller "Touch1"))
  (bind (_worldlocation _worlddirection) (Game|Player|ConvertMouseLocationToWorldSpace _playercontroller))
  (bind _returnvalue_5 (/ _roomsize 2))
  (bind (_x _y) (Math|Vector|BreakVector _returnvalue_5))
  (bind (_worldposition _worlddirection_2) (Class|GameplayStatics|DeprojectScreentoWorld _playercontroller (Math|Vector2D|MakeVector2D _locationx _locationy)))
  (bind _returnvalue_6 (* _returnvalue_5 -1))
  (bind (_x_2 _y_2) (Math|Vector|BreakVector _returnvalue_6))
  (LocalVariables|SetCameraLocation (Camera|GetCameraLocation (Variables|/Script/Engine.PlayerController|GetPlayerCameraManager _playercontroller)))
  (LocalVariables|SetMouseLocation (Math|Vector|SelectVector (+ _worldposition (* _worlddirection_2 500000)) (+ _worldlocation (* _worlddirection 500000)) _biscurrentlypressed))
  (return (Math|Vector|SelectVector (Math|Vector|SelectVector (.Intersection (Class|KismetMathLibrary|LinePlaneIntersectionOriginNormal (LocalVariables|GetCameraLocation) (LocalVariables|GetMouseLocation) (Math|Vector|MakeVector _x 0.0 0.0) _returnvalue_4)) (.Intersection (Class|KismetMathLibrary|LinePlaneIntersectionOriginNormal (LocalVariables|GetCameraLocation) (LocalVariables|GetMouseLocation) (Math|Vector|MakeVector _x_2 0.0 0.0) _returnvalue_3)) (> (.T (Class|KismetMathLibrary|LinePlaneIntersectionOriginNormal (LocalVariables|GetCameraLocation) (LocalVariables|GetMouseLocation) (Math|Vector|MakeVector _x 0.0 0.0) _returnvalue_4)) (.T (Class|KismetMathLibrary|LinePlaneIntersectionOriginNormal (LocalVariables|GetCameraLocation) (LocalVariables|GetMouseLocation) (Math|Vector|MakeVector _x_2 0.0 0.0) _returnvalue_3)))) (Math|Vector|SelectVector (.Intersection (Class|KismetMathLibrary|LinePlaneIntersectionOriginNormal (LocalVariables|GetCameraLocation) (LocalVariables|GetMouseLocation) (Math|Vector|MakeVector 0.0 _y 0.0) _returnvalue)) (.Intersection (Class|KismetMathLibrary|LinePlaneIntersectionOriginNormal (LocalVariables|GetCameraLocation) (LocalVariables|GetMouseLocation) (Math|Vector|MakeVector 0.0 _y_2 0.0) _returnvalue_2)) (> (.T (Class|KismetMathLibrary|LinePlaneIntersectionOriginNormal (LocalVariables|GetCameraLocation) (LocalVariables|GetMouseLocation) (Math|Vector|MakeVector 0.0 _y 0.0) _returnvalue)) (.T (Class|KismetMathLibrary|LinePlaneIntersectionOriginNormal (LocalVariables|GetCameraLocation) (LocalVariables|GetMouseLocation) (Math|Vector|MakeVector 0.0 _y_2 0.0) _returnvalue_2)))) (< (Class|KismetMathLibrary|VectorDistanceSquared (Math|Vector|SelectVector (.Intersection (Class|KismetMathLibrary|LinePlaneIntersectionOriginNormal (LocalVariables|GetCameraLocation) (LocalVariables|GetMouseLocation) (Math|Vector|MakeVector _x 0.0 0.0) _returnvalue_4)) (.Intersection (Class|KismetMathLibrary|LinePlaneIntersectionOriginNormal (LocalVariables|GetCameraLocation) (LocalVariables|GetMouseLocation) (Math|Vector|MakeVector _x_2 0.0 0.0) _returnvalue_3)) (> (.T (Class|KismetMathLibrary|LinePlaneIntersectionOriginNormal (LocalVariables|GetCameraLocation) (LocalVariables|GetMouseLocation) (Math|Vector|MakeVector _x 0.0 0.0) _returnvalue_4)) (.T (Class|KismetMathLibrary|LinePlaneIntersectionOriginNormal (LocalVariables|GetCameraLocation) (LocalVariables|GetMouseLocation) (Math|Vector|MakeVector _x_2 0.0 0.0) _returnvalue_3)))) (LocalVariables|GetCameraLocation)) (Class|KismetMathLibrary|VectorDistanceSquared (LocalVariables|GetCameraLocation) (Math|Vector|SelectVector (.Intersection (Class|KismetMathLibrary|LinePlaneIntersectionOriginNormal (LocalVariables|GetCameraLocation) (LocalVariables|GetMouseLocation) (Math|Vector|MakeVector 0.0 _y 0.0) _returnvalue)) (.Intersection (Class|KismetMathLibrary|LinePlaneIntersectionOriginNormal (LocalVariables|GetCameraLocation) (LocalVariables|GetMouseLocation) (Math|Vector|MakeVector 0.0 _y_2 0.0) _returnvalue_2)) (> (.T (Class|KismetMathLibrary|LinePlaneIntersectionOriginNormal (LocalVariables|GetCameraLocation) (LocalVariables|GetMouseLocation) (Math|Vector|MakeVector 0.0 _y 0.0) _returnvalue)) (.T (Class|KismetMathLibrary|LinePlaneIntersectionOriginNormal (LocalVariables|GetCameraLocation) (LocalVariables|GetMouseLocation) (Math|Vector|MakeVector 0.0 _y_2 0.0) _returnvalue_2))))))) (Math|Vector|SelectVector (Math|Vector|SelectVector _returnvalue_4 _returnvalue_3 (> (.T (Class|KismetMathLibrary|LinePlaneIntersectionOriginNormal (LocalVariables|GetCameraLocation) (LocalVariables|GetMouseLocation) (Math|Vector|MakeVector _x 0.0 0.0) _returnvalue_4)) (.T (Class|KismetMathLibrary|LinePlaneIntersectionOriginNormal (LocalVariables|GetCameraLocation) (LocalVariables|GetMouseLocation) (Math|Vector|MakeVector _x_2 0.0 0.0) _returnvalue_3)))) (Math|Vector|SelectVector _returnvalue _returnvalue_2 (> (.T (Class|KismetMathLibrary|LinePlaneIntersectionOriginNormal (LocalVariables|GetCameraLocation) (LocalVariables|GetMouseLocation) (Math|Vector|MakeVector 0.0 _y 0.0) _returnvalue)) (.T (Class|KismetMathLibrary|LinePlaneIntersectionOriginNormal (LocalVariables|GetCameraLocation) (LocalVariables|GetMouseLocation) (Math|Vector|MakeVector 0.0 _y_2 0.0) _returnvalue_2)))) (< (Class|KismetMathLibrary|VectorDistanceSquared (Math|Vector|SelectVector (.Intersection (Class|KismetMathLibrary|LinePlaneIntersectionOriginNormal (LocalVariables|GetCameraLocation) (LocalVariables|GetMouseLocation) (Math|Vector|MakeVector _x 0.0 0.0) _returnvalue_4)) (.Intersection (Class|KismetMathLibrary|LinePlaneIntersectionOriginNormal (LocalVariables|GetCameraLocation) (LocalVariables|GetMouseLocation) (Math|Vector|MakeVector _x_2 0.0 0.0) _returnvalue_3)) (> (.T (Class|KismetMathLibrary|LinePlaneIntersectionOriginNormal (LocalVariables|GetCameraLocation) (LocalVariables|GetMouseLocation) (Math|Vector|MakeVector _x 0.0 0.0) _returnvalue_4)) (.T (Class|KismetMathLibrary|LinePlaneIntersectionOriginNormal (LocalVariables|GetCameraLocation) (LocalVariables|GetMouseLocation) (Math|Vector|MakeVector _x_2 0.0 0.0) _returnvalue_3)))) (LocalVariables|GetCameraLocation)) (Class|KismetMathLibrary|VectorDistanceSquared (LocalVariables|GetCameraLocation) (Math|Vector|SelectVector (.Intersection (Class|KismetMathLibrary|LinePlaneIntersectionOriginNormal (LocalVariables|GetCameraLocation) (LocalVariables|GetMouseLocation) (Math|Vector|MakeVector 0.0 _y 0.0) _returnvalue)) (.Intersection (Class|KismetMathLibrary|LinePlaneIntersectionOriginNormal (LocalVariables|GetCameraLocation) (LocalVariables|GetMouseLocation) (Math|Vector|MakeVector 0.0 _y_2 0.0) _returnvalue_2)) (> (.T (Class|KismetMathLibrary|LinePlaneIntersectionOriginNormal (LocalVariables|GetCameraLocation) (LocalVariables|GetMouseLocation) (Math|Vector|MakeVector 0.0 _y 0.0) _returnvalue)) (.T (Class|KismetMathLibrary|LinePlaneIntersectionOriginNormal (LocalVariables|GetCameraLocation) (LocalVariables|GetMouseLocation) (Math|Vector|MakeVector 0.0 _y_2 0.0) _returnvalue_2)))))))))

(fn MoveElement
  (params (Element :type BP%20World%20Element%20Object%20Reference))
  (bind (_location _normal) (CallFunction|GetMouseLocation))
  (bind _angle (Private|GetRotation _normal))
  (bind _rotatedlocation (Private|GetRotatedLocation _location _angle))
  (bind _position (Private|GetValidRoomPosition Element _rotatedlocation _normal))
  (bind _returnvalue (Private|GetClosestGridPosition Element _position _normal))
  (Transformation|SetActorLocation Element _returnvalue false true)
  (Transformation|SetActorRotation Element (Math|Conversions|RotationFromXVector _normal)))

(fn CalculateOffset
  (params (Element :type BP%20World%20Element%20Object%20Reference))
  (bind (_location _normal) (CallFunction|GetMouseLocation))
  (Variables|Private|SetOffset (- (Transformation|GetActorLocation Element) _location))
  (Variables|Private|SetNormal _normal))

(fn SetInitialLocation
  (params (Element :type BP%20World%20Element%20Object%20Reference))
  (bind (_location _normal) (CallFunction|GetMouseLocation))
  (bind _position (Private|GetValidRoomPosition Element _location _normal))
  (bind _returnvalue (Private|GetClosestGridPosition Element _position _normal))
  (Transformation|SetActorLocation Element _returnvalue false true)
  (Transformation|SetActorRotation Element (Math|Conversions|RotationFromXVector _normal)))

(fn GetClosestGridPosition
  (params (Element :type BP%20World%20Element%20Object%20Reference) (Initial :type Vector) (NewNormal :type Vector))
  (bind (_x _y _z) (Math|Vector|BreakVector Initial))
  (bind _returnvalue (Class|KismetMathLibrary|VectorRight))
  (bind _horizontalgridsize (Variables|Private|GetHorizontalGridSize))
  (bind _returnvalue_2 (Math|Vector|VectorGetAbs NewNormal))
  (bind _returnvalue_3 (/ _horizontalgridsize 2))
  (bind _elementinfo (Variables|/Game/Juaner/Blueprints/BP_WorldElement.BP_WorldElement_C|GetElementInfo Element))
  (bind _returnvalue_4 (Utilities|Operators|EqualEqual _returnvalue_2 _returnvalue 0.0))
  (bind _size (Variables|/Game/Juaner/Elements/DA_ElementInfo.DA_ElementInfo_C|GetSize _elementinfo))
  (bind _returnvalue_5 (Utilities|Select :Index _size :NewEnumerator2 0.0 :NewEnumerator0 0.0 :NewEnumerator1 _returnvalue_3))
  (bind _returnvalue_6 (Math|Float|SelectFloat 0.0 _returnvalue_5 _returnvalue_4))
  (bind _returnvalue_7 (Math|Float|SelectFloat _returnvalue_5 0.0 _returnvalue_4))
  (return (Math|Vector|MakeVector (+ (* (Math|Float|Round (/ (- _x _returnvalue_7) (Variables|Private|GetHorizontalGridSize))) (Variables|Private|GetHorizontalGridSize)) _returnvalue_7) (+ (* (Math|Float|Round (/ (- _y _returnvalue_6) (Variables|Private|GetHorizontalGridSize))) (Variables|Private|GetHorizontalGridSize)) _returnvalue_6) (* (Math|Float|Round (/ _z (Variables|Private|GetVerticalGridSize))) (Variables|Private|GetVerticalGridSize)))))

(fn SetRoomSize
  (params (RoomSize :type Vector))
  (Variables|Private|SetRoomSize RoomSize))

(fn GetRotatedLocation
  (params (Location :type Vector) (Angle :type Float%20%28double-precision%29))
  (return (+ Location (Math|Vector|RotateVectorAroundAxis (Variables|Private|GetOffset) Angle (Math|Vector|VectorUp)))))

(fn GetRotation
  (params (NewNormal :type Vector))
  (bind _normal (Variables|Private|GetNormal))
  (return (Class|KismetMathLibrary|DegAtan2 (Math|Vector|DotProduct (Math|Vector|CrossProduct _normal NewNormal) (Math|Vector|VectorUp)) (Math|Vector|DotProduct NewNormal _normal))))

(fn Initialize
  (params (HorizontalGridSize :type Float%20%28double-precision%29) (VerticalGridSize :type Float%20%28double-precision%29))
  (Variables|Private|SetHorizontalGridSize HorizontalGridSize)
  (Variables|Private|SetVerticalGridSize VerticalGridSize))